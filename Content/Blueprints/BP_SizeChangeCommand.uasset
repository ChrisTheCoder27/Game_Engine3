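; BP_SizeChangeCommand is a command Blueprint that changes the size of a BP_Receiver actor.
; Its Execute event logs, casts TargetActor to BP_Receiver, then sets its scale to double or normal based on the receiver's IncreaseSize flag.
; The follow-up casts have no input and the nodes that would flip the flag are unconnected, so this graph never toggles it.
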(event EventExecute
  (bind _targetactor (Variables|Default|GetTargetActor))
  (Development|PrintString "Execute fired")
  (Utilities|IsValid _targetactor
    (:Is%20Valid
      (bind _asbp_receiver (Utilities|Casting|CastToBP_Receiver _targetactor))
      (if (Variables|/Game/Blueprints/BP_Receiver.BP_Receiver_C|GetIncreaseSize _asbp_receiver)
        (Transformation|SetActorScale3D _asbp_receiver "2.000000,2.000000,2.000000")
        (bind _asbp_receiver_2 (Utilities|Casting|CastToBP_Receiver))
        (else
          (Transformation|SetActorScale3D _asbp_receiver "1.000000,1.000000,1.000000")
          (bind _asbp_receiver_3 (Utilities|Casting|CastToBP_Receiver)))))))

(fn ConstructionScript)